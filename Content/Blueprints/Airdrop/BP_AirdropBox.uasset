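; Airdrop crate that descends under physics with a parachute, which a timeline scales open on BeginPlay.
; After a short delay, Tick watches for zero vertical velocity on the box to detect landing.
; Landing freezes physics, swaps the parachute for temporary smoke, and loops over ItemsInfo to gather each item's data.
; That loop casts to the battle-royale player controller but ends in an empty sequence, so no items spawn here.
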(event `self.ReceiveBeginPlay`
  (bind (_direction _value) (`Timeline|TL_OpenParachute` :!via `PlayFromStart`)
    (:`Update`
      (`SceneComponent.SetRelativeScale3D` (`self.Parachute`) (`KismetMathLibrary.Conv_DoubleToVector` _value))
      (`KismetSystemLibrary.Delay` 1.0)
      (set `self.CanTick` true))))

(event `self.ReceiveTick`
  (params (DeltaSeconds :type "Float (single-precision)"))
  (bind (_returnvalue_x _returnvalue_y _returnvalue_z) (`KismetMathLibrary.BreakVector` (`SceneComponent.GetComponentVelocity` (`self.Box`))))
  (if (`self.CanTick`)
    ;[1 0 0.09375] Checking the Landing
    (if (== _returnvalue_z 0.0)
      (set `self.CanTick` false)
      (`|ExecutionSequence`
        (:`then_0`
          ;[0 1 0.9766] Turn off physical function
          (`PrimitiveComponent.SetSimulatePhysics` (`self.Box`) false)
          (`KismetSystemLibrary.Delay` 0.2)
          ;[0 1 0.9063] Remove the parachute and start playing smoke
          (`ActorComponent.K2_DestroyComponent` (`self.Parachute`))
          (`ActorComponent.SetActive` (`self.Smoke`) true true)
          ;[0.3359 0 1] Delete the smoke after it has lasted for a while
          (`KismetSystemLibrary.Delay` 10.0)
          (`ActorComponent.K2_DestroyComponent` (`self.Smoke`)))
        (:`then_1`
          (for _array_element (`self.ItemsInfo`)
            (set `self.ItemTransform` (`KismetMathLibrary.MakeTransform` (`self.K2_GetActorLocation`)))
            (bind (_sn _itemtype _id _amount) (break `/Game/Blueprints/Datas/TableStructure/Airdrop/AirdropBoxItem` _array_element))
            (set `self.ItemSN` _sn)
            (set `self.ItemID` _id)
            (set `self.ItemAmount` _amount)
            (set `self.As PC Battle Royale` (cast `/Game/Blueprints/Gameplay/PC_BattleRoyale` (`GameplayStatics.GetPlayerController` 0) :!pure true))
            (`|ExecutionSequence`)))))))

(fn `UserConstructionScript`)