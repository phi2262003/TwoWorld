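; Airdrop plane that flies from a start point to a drop point, releases a supply box, then flies away.
; The construction script calls StartToAirdrop, which places the plane at the start, facing the drop point.
; Two chained timelines, sized by distance over airspeed, lerp its position for constant-speed legs.
; Between legs it spawns BP_AirdropBox with its item info, then continues far along its heading and destroys itself.
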(event `StartToAirdrop`
  (bind _returnvalue (/ (`KismetMathLibrary.VSize` (- (`self.DropPoint`) (`self.EndPoint`))) (`self.Airspeed`)))
  (bind _returnvalue_2 (/ (`KismetMathLibrary.VSize` (- (`self.StartPoint`) (`self.DropPoint`))) (`self.Airspeed`)))
  (`|ExecutionSequence`
    (:`then_0`
      ;[0 1 0.7656] Set the initial position and direction of the airplane
      (`self.K2_SetActorLocation` (`self.StartPoint`))
      (`self.K2_SetActorRotation` (`KismetMathLibrary.FindLookAtRotation` (`self.StartPoint`) (`self.DropPoint`))))
    (:`then_1`
      ;[0 0.6484 1] Flying from the starting point to the throwing point
      (`TimelineComponent.SetTimelineLength` (`self.TL_Fly 1`) _returnvalue_2)
      (bind (_direction _value) (`Timeline|TL_Fly 1` :!via `PlayFromStart`)
        (:`Update`
          (`self.K2_SetActorLocation` (`KismetMathLibrary.VLerp` (`self.StartPoint`) (`self.DropPoint`) (/ _value _returnvalue_2))))
        (:`Finished`
          ;[0 0.4844 1] Spawm Airdrop Box
          (`|SpawnActorFromClass` "/Game/Blueprints/Airdrop/BP_AirdropBox.BP_AirdropBox_C" (`self.GetTransform`) "Undefined" "OverrideRootScale" null (`self.ItemInfo`) null)
          ;[0 0.8125 1] Calculate the end of flight
          (set `self.EndPoint` (+ (`self.DropPoint`) (* (`self.GetActorForwardVector`) 500000.0)))
          ;[0.1484 0 1] Flying from the throwing point to the end
          (`TimelineComponent.SetTimelineLength` (`self.TL_Fly 2`) _returnvalue)
          (bind (_direction_2 _value_2) (`Timeline|TL_Fly 2` :!via `PlayFromStart`)
            (:`Update`
              (`self.K2_SetActorLocation` (`KismetMathLibrary.VLerp` (`self.DropPoint`) (`self.EndPoint`) (/ _value_2 _returnvalue))))
            (:`Finished`
              (`self.K2_DestroyActor`))))))))

(fn `UserConstructionScript`
  (`self.StartToAirdrop`))