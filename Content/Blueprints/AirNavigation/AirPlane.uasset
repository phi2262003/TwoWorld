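; Airplane actor that flies in a straight line from StartPoint to EndPoint at FlyingSpeed, then destroys itself.
; The construction script calls StartFlying, which places the plane at the start facing the end and sets the timeline length to distance over speed.
; Each timeline update lerps the position by track value over duration, passing it to OnFlying before moving the actor.
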(event `StartFlying`
  (bind _returnvalue (/ (`KismetMathLibrary.VSize` (- (`self.StartPoint`) (`self.EndPoint`))) (`self.FlyingSpeed`)))
  (`|ExecutionSequence`
    (:`then_0`
      ;[1 0.3047 0] Set the initial direction and position of the aircraft
      (`self.K2_SetActorRotation` (`KismetMathLibrary.FindLookAtRotation` (`self.StartPoint`) (`self.EndPoint`)))
      (`self.K2_SetActorLocation` (`self.StartPoint`)))
    (:`then_1`
      ;[1 0.2578 0] Control the flight with Timeline
      (`TimelineComponent.SetTimelineLength` (`self.Timeline_Flying`) _returnvalue)
      (bind (_direction _newtrack_0) (`Timeline|Timeline_Flying`)
        (:`Update`
          (bind _returnvalue_2 (`KismetMathLibrary.VLerp` (`self.StartPoint`) (`self.EndPoint`) (/ _newtrack_0 _returnvalue)))
          (`self.OnFlying` _returnvalue_2)
          (`self.K2_SetActorLocation` _returnvalue_2))
        (:`Finished`
          (`self.K2_DestroyActor`))))))

(fn `UserConstructionScript`
  (`self.StartFlying`))