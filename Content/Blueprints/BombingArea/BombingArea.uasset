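; BombingArea is an actor that sets off a timed bombing run over predefined points.
; After a start delay, Tick accumulates elapsed time and scans BombDatas for an entry whose BlastTime has passed.
; For that entry it line-traces straight down at the point's X/Y and spawns a BlastPoint at the hit location, handling one bomb per frame.
; Once the list is empty it destroys itself after a short delay.
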(event `self.ReceiveBeginPlay`
  (`KismetSystemLibrary.Delay` (`self.DelayTime`))
  (set `self.Start` true))

(event `self.ReceiveTick`
  (params (DeltaSeconds :type "Float (single-precision)"))
  (if (`self.Start`)
    (set `self.Duration` (+ DeltaSeconds (`self.Duration`)))
    (if (> (`KismetArrayLibrary.Array_Length` (`self.BombDatas`)) 0)
      ;[1 0 0.09375] Loop all the bomb information to find the point where it can blast
      (for (_array_element _array_index) (`self.BombDatas`)
        (bind (_point _blasttime) (break `/Game/Blueprints/Datas/TableStructure/ST_BombZone` _array_element))
        (if (>= (`self.Duration`) _blasttime)
          (bind _x (.x _point))
          (bind _y (.y _point))
          ;[1 0.09375 0] Make a ray collision downwards from a specified position and blast when it hits a collision-able object
          (bind _outhit (`KismetSystemLibrary.LineTraceSingle` (`KismetMathLibrary.MakeVector` _x _y 100000.0) (`KismetMathLibrary.MakeVector` _x _y -100000.0) "TraceTypeQuery1"))
          (`|SpawnActorFromClass` "/Game/Blueprints/BombingArea/BlastPoint.BlastPoint_C" (`KismetMathLibrary.MakeTransform` (`.Location` (`GameplayStatics.BreakHitResult` _outhit))) "Undefined" "OverrideRootScale" null null)
          (`KismetArrayLibrary.Array_Remove` (`self.BombDatas`) _array_index)
          (break)))
      (else
        (`KismetSystemLibrary.Delay` 0.5)
        (`self.K2_DestroyActor`)))))

(fn `UserConstructionScript`)