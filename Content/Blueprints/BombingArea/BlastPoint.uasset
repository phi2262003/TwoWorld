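; BlastPoint is a short-lived explosion actor for the bombing area that reports player hits.
; Sphere overlaps pass through a gate that starts open and closes 0.1 seconds after BeginPlay, limiting hits to the initial blast.
; An overlapping local player triggers CharacterTouchedBomb on PC_BattleRoyale with the distance to the blast.
; The actor lingers about four seconds, then destroys itself.
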(event `self.ReceiveBeginPlay`
  (bind _returnvalue (`GameplayStatics.GetPlayerCharacter` 0))
  (`KismetSystemLibrary.Delay` 0.1)
  (`|ExecutionSequence`
    (:`then_0`
      (`KismetSystemLibrary.Delay` 4.0)
      (`self.K2_DestroyActor`))
    (:`then_1`
      (goto _label :!via `Close`))))

(event `self.Sphere.OnComponentBeginOverlap`
  (params (OverlappedComponent :type "PrimitiveComponent Object Reference") (OtherActor :type "Actor Object Reference") (OtherComp :type "PrimitiveComponent Object Reference") (OtherBodyIndex :type Integer) (bFromSweep :type Boolean) (SweepResult :type "HitResult Structure (by ref)"))
  (bind _returnvalue (`GameplayStatics.GetPlayerCharacter` 0))
  (`/Engine/EditorBlueprintResources/StandardMacros.Gate` false :!label _label
    (:`Exit`
      (if (== OtherActor _returnvalue)
        (`/Game/Blueprints/Gameplay/PC_BattleRoyale.CharacterTouchedBomb` (cast `/Game/Blueprints/Gameplay/PC_BattleRoyale` (`GameplayStatics.GetPlayerController` 0) :!pure true) (`KismetMathLibrary.VSize` (- (`self.K2_GetActorLocation` _returnvalue) (`self.K2_GetActorLocation`))))))))

(fn `UserConstructionScript`)