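; Player character for the battle royale game, with modular clothing, visible weapons and equipment, and stance-based montages.
; Clothing meshes follow the body via leader pose, swapping from a fashion DataTable with mask textures on a dynamic skin material and default fallbacks.
; Display functions read PlayerState to socket guns and gear, shifting back weapons for backpacks and hiding hair under helmets.
; A timeline offsets the camera for hold-aiming.
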(event `self.ReceiveBeginPlay`
  ;[1 0.6328 0] Enhanced Input
  (bind _aspc_battle_royale (cast `/Game/Blueprints/Gameplay/PC_BattleRoyale` (`self.GetController`)))
  (bind _output_get (set `self.As PC Battle Royale` _aspc_battle_royale))
  (`EnhancedInputSubsystemInterface.AddMappingContext` (pcsubsystem `EnhancedInputLocalPlayerSubsystem` _output_get) "/Game/Blueprints/Input/IMC_Player.IMC_Player" 0 (struct))
  ;[1 0.8438 0] Create object REF
  (bind _asps_battle_royale (cast `/Game/Blueprints/Gameplay/PS_BattleRoyale` (`self.PlayerState`)))
  (set `self.As PS Battle Royale` _asps_battle_royale)
  (bind _asgi_battle_royale (cast `/Game/Blueprints/Gameplay/GI_BattleRoyale` (`GameplayStatics.GetGameInstance`)))
  (set `self.As GI Battle Royale` _asgi_battle_royale))

(event `HoldAiming`
  (params (Forward :type Boolean))
  (if Forward
    (bind (_direction _percent) (`Timeline|TL_HoldAiming` :!label _label)
      (:`Update`
        (`SceneComponent.K2_SetRelativeLocation` (`self.Camera`) (`KismetMathLibrary.VLerp` (0.0 0.0 0.0) (100.0 5.0 -30.0) _percent) false false)))
    (else
      (goto _label :!via `Reverse`))))

(fn `Attach`
  (params (Item :type "/Game/Blueprints/Items/ItemBase Object Reference") (SocketName :type Name))
  (`self.K2_SetActorTransform` (`local.Item`) (`SceneComponent.GetSocketTransform` (`self.Mesh`) (`local.SocketName`) "RTS_World") false false)
  (`self.K2_AttachToComponent` (`local.Item`) (`self.Mesh`) (`local.SocketName`) "SnapToTarget" "KeepWorld" "KeepRelative" true))

(fn `ClearFashion`
  (`self.ReplaceSkeletalMesh` "NewEnumerator0" "0")
  (`self.ReplaceSkeletalMesh` "NewEnumerator1" "0")
  (`self.ReplaceSkeletalMesh` "NewEnumerator2" "0")
  (`self.ReplaceSkeletalMesh` "NewEnumerator3" "0"))

(fn `GetCurrentMontages`
  (returns (ReturnValue :type "AnimMontage Object Reference"))
  (return null))

(fn `GetFashionDatas`
  (params (ID :type Name))
  (returns (SkeletalMesh :type "SkeletalMesh Object Reference") (MaskTexture :type "Texture Object Reference"))
  (bind _returnvalue (`|GetDataTableRow` "/Game/Blueprints/Datas/DataTable/Items/DT_Item_Fashion.DT_Item_Fashion" ID)
    (:`then`
      (bind (_type _name _icon _skeletalmesh _staticmesh _masktexture) (break `/Game/Blueprints/Datas/TableStructure/Items/ST_Items_Fashion` _returnvalue))
      (return _skeletalmesh _masktexture))
    (:`RowNotFound`
      (return null null))))

(fn `InitSkeletalMesh`
  (`|ExecutionSequence`
    (:`then_0`
      ;[0 0.08594 1] Create Skin Material
      (bind _returnvalue (`KismetMaterialLibrary.CreateDynamicMaterialInstance` "/Game/Assets/Humans/Female/Materials/Skin/M_MT_Skin.M_MT_Skin"))
      (bind _output_get (set `self.SkinMatRef` _returnvalue))
      (`PrimitiveComponent.SetMaterialByName` (`self.Mesh`) "skin" _output_get))
    (:`then_1`
      ;[0.9922 0 1] Set Leader Pose
      (`SkinnedMeshComponent.SetLeaderPoseComponent` (`self.SKM_UnderwearTop`) (`self.Mesh`) false false)
      (`SkinnedMeshComponent.SetLeaderPoseComponent` (`self.SKM_UnderwearBottom`) (`self.Mesh`) false false)
      (`SkinnedMeshComponent.SetLeaderPoseComponent` (`self.SKM_ClothTop`) (`self.Mesh`) false false)
      (`SkinnedMeshComponent.SetLeaderPoseComponent` (`self.SKM_ClothBottom`) (`self.Mesh`) false false)
      (`SkinnedMeshComponent.SetLeaderPoseComponent` (`self.SKM_Whole`) (`self.Mesh`) false false)
      (`SkinnedMeshComponent.SetLeaderPoseComponent` (`self.SKM_Shoes`) (`self.Mesh`) false false))
    (:`then_2`
      ;[0.5469 0 1] Attach Hair
      (`SceneComponent.K2_AttachToComponent` (`self.SKM_Hair`) (`self.Mesh`) "head" "KeepWorld" "KeepWorld" "KeepWorld" true))
    (:`then_3`
      ;[0.4297 0 1] Init SkeletalMesh
      (`self.ReplaceSkeletalMesh` "NewEnumerator0" "0"))))

(fn `MouseLookUp`
  (params (AxisValue :type "Float (double-precision)"))
  (`self.AddControllerPitchInput` AxisValue))

(fn `MouseTurn`
  (params (AxisValue :type "Float (double-precision)"))
  (`self.AddControllerYawInput` AxisValue))

(fn `PlayMontage`
  (params (MontageType :type "/Game/Blueprints/Datas/Enum/E_MontageType Enum" :default "NewEnumerator0"))
  (set `self.PlayingMontageType` MontageType)
  (set `self.IsPlayingMontage` true)
  (if (`self.IsProne`)
    ;[0.5469 1 0] Prone montage animation
    (switch `/Game/Blueprints/Datas/Enum/E_MontageType` (`local.MontageType`)
      (:`NewEnumerator0`
        (`self.PlayAnimMontage` "/Game/Blueprints/Character/AnimationMontage/AM_Prone_Equip.AM_Prone_Equip"))
      (:`NewEnumerator1`
        (`self.PlayAnimMontage` "/Game/Blueprints/Character/AnimationMontage/AM_Prone_UnEquip.AM_Prone_UnEquip"))
      (:`NewEnumerator2`
        (`self.PlayAnimMontage` "/Game/Blueprints/Character/AnimationMontage/AM_Prone_Reload.AM_Prone_Reload"))
      (:`NewEnumerator3`
        (`self.PlayAnimMontage` "/Game/Blueprints/Character/AnimationMontage/AM_Prone_Reload.AM_Prone_Reload" 1.0 "ReloadBullet"))
      (:`NewEnumerator4`
        (`self.PlayAnimMontage` "/Game/Blueprints/Character/AnimationMontage/AM_Rifle_Prone_Fire.AM_Rifle_Prone_Fire"))
      (:`NewEnumerator5`
        (`self.PlayAnimMontage` "/Game/Blueprints/Character/AnimationMontage/AM_Prone_Use_Bandage.AM_Prone_Use_Bandage")))
    (elif (`self.IsCrouching`)
      ;[0.9688 1 0] Crouch montage animation
      (switch `/Game/Blueprints/Datas/Enum/E_MontageType` (`local.MontageType`)
        (:`NewEnumerator0`
          (`self.PlayAnimMontage` "/Game/Blueprints/Character/AnimationMontage/AM_Crouch_Equip.AM_Crouch_Equip"))
        (:`NewEnumerator1`
          (`self.PlayAnimMontage` "/Game/Blueprints/Character/AnimationMontage/AM_Crouch_UnEquip.AM_Crouch_UnEquip"))
        (:`NewEnumerator2`
          (`self.PlayAnimMontage` "/Game/Blueprints/Character/AnimationMontage/AM_Stand_Reload.AM_Stand_Reload"))
        (:`NewEnumerator3`
          (`self.PlayAnimMontage` "/Game/Blueprints/Character/AnimationMontage/AM_Stand_Reload.AM_Stand_Reload" 1.0 "ReloadBullet"))
        (:`NewEnumerator4`
          (`self.PlayAnimMontage` "/Game/Blueprints/Character/AnimationMontage/AM_Rifle_Crouch_Fire.AM_Rifle_Crouch_Fire"))
        (:`NewEnumerator5`
          (`self.PlayAnimMontage` "/Game/Blueprints/Character/AnimationMontage/AM_Crouch_Use_Bandage.AM_Crouch_Use_Bandage")))
      (else
        ;[0.9688 0 1] Stand Montage Animation
        (switch `/Game/Blueprints/Datas/Enum/E_MontageType` (`local.MontageType`)
          (:`NewEnumerator0`
            (`self.PlayAnimMontage` "/Game/Blueprints/Character/AnimationMontage/AM_Stand_Equip.AM_Stand_Equip"))
          (:`NewEnumerator1`
            (`self.PlayAnimMontage` "/Game/Blueprints/Character/AnimationMontage/AM_Stand_UnEquip.AM_Stand_UnEquip"))
          (:`NewEnumerator2`
            (`self.PlayAnimMontage` "/Game/Blueprints/Character/AnimationMontage/AM_Stand_Reload.AM_Stand_Reload"))
          (:`NewEnumerator3`
            (`self.PlayAnimMontage` "/Game/Blueprints/Character/AnimationMontage/AM_Stand_Reload.AM_Stand_Reload" 1.0 "ReloadBullet"))
          (:`NewEnumerator4`
            (`self.PlayAnimMontage` "/Game/Blueprints/Character/AnimationMontage/AM_Rifle_Stand_Fire.AM_Rifle_Stand_Fire"))
          (:`NewEnumerator5`
            (`self.PlayAnimMontage` "/Game/Blueprints/Character/AnimationMontage/AM_Stand_Use_Bandage.AM_Stand_Use_Bandage")))))))

(fn `ReplaceSkeletalMesh`
  (params (FashionType :type "/Game/Blueprints/Datas/Enum/E_FashionType Enum" :default "NewEnumerator0") (Name :type Name))
  (locals (SKM :type "SkeletalMesh Object Reference") (Mask :type "Texture Object Reference"))
  (bind _skm (`local.SKM`))
  (bind _skm_2 (`local.SKM`))
  (bind _skm_3 (`local.SKM`))
  (`|ExecutionSequence`
    (:`then_0`
      (bind (_skeletalmesh _masktexture) (`self.GetFashionDatas` Name))
      (set `local.SKM` _skeletalmesh)
      (set `local.Mask` _masktexture)
      ;[0 1 0.9766] Replace Skeletal Mesh
      (switch `/Game/Blueprints/Datas/Enum/E_FashionType` FashionType
        (:`NewEnumerator0`
          (`SkeletalMeshComponent.SetSkeletalMeshAsset` (`self.SKM_ClothTop`) _skm)
          ;[1 0 0.5625] Set Mask
          (`MaterialInstanceDynamic.SetTextureParameterValue` (`self.SkinMatRef`) "Mask  Top" (`local.Mask`))
          ;[0.4531 1 0] Whole Special Modify
          (if (!= _skm null)
            (`SkeletalMeshComponent.SetSkeletalMeshAsset` (`self.SKM_Whole`) null)))
        (:`NewEnumerator1`
          (`SkeletalMeshComponent.SetSkeletalMeshAsset` (`self.SKM_ClothBottom`) _skm_2)
          (`MaterialInstanceDynamic.SetTextureParameterValue` (`self.SkinMatRef`) "Mask  Bottom" (`local.Mask`))
          (if (!= _skm_2 null)
            (`SkeletalMeshComponent.SetSkeletalMeshAsset` (`self.SKM_Whole`) null)))
        (:`NewEnumerator2`
          (`SkeletalMeshComponent.SetSkeletalMeshAsset` (`self.SKM_Whole`) _skm_3)
          (`MaterialInstanceDynamic.SetTextureParameterValue` (`self.SkinMatRef`) "Mask Top" (`local.Mask`))
          (if (!= _skm_3 null)
            (`SkeletalMeshComponent.SetSkeletalMeshAsset` (`self.SKM_ClothTop`) null)
            (`SkeletalMeshComponent.SetSkeletalMeshAsset` (`self.SKM_ClothBottom`) null)))
        (:`NewEnumerator3`
          (`SkeletalMeshComponent.SetSkeletalMeshAsset` (`self.SKM_Shoes`) (`local.SKM`))
          (`/Engine/EditorBlueprintResources/StandardMacros.IsValid` (`local.SKM`)
            (:`Is Valid`
              (`MaterialInstanceDynamic.SetTextureParameterValue` (`self.SkinMatRef`) "Mask Foot" (`local.Mask`)))
            (:`Is Not Valid`
              (`MaterialInstanceDynamic.SetTextureParameterValue` (`self.SkinMatRef`) "Mask Foot" "/Game/Assets/Humans/Female/Textures/System/TX_Empty_white.TX_Empty_white"))))))
    (:`then_1`
      ;[1 0.8203 0] Set the default SkeletalMesh and Mask
      (`/Engine/EditorBlueprintResources/StandardMacros.IsValid` (`SkeletalMeshComponent.SkeletalMeshAsset` (`self.SKM_Whole`))
        (:`Is Valid`
          (`MaterialInstanceDynamic.SetTextureParameterValue` (`self.SkinMatRef`) "Mask Bottom" "/Game/Assets/Humans/Female/Textures/System/TX_Empty_white.TX_Empty_white"))
        (:`Is Not Valid`
          (`|ExecutionSequence`
            (:`then_0`
              (`/Engine/EditorBlueprintResources/StandardMacros.IsValid` (`SkeletalMeshComponent.SkeletalMeshAsset` (`self.SKM_ClothTop`))
                (:`Is Not Valid`
                  (bind (_skeletalmesh_2 _masktexture_2) (`self.GetFashionDatas` "1"))
                  (`SkeletalMeshComponent.SetSkeletalMeshAsset` (`self.SKM_ClothTop`) _skeletalmesh_2)
                  (`MaterialInstanceDynamic.SetTextureParameterValue` (`self.SkinMatRef`) "Mask Top" _masktexture_2))))
            (:`then_1`
              (`/Engine/EditorBlueprintResources/StandardMacros.IsValid` (`SkeletalMeshComponent.SkeletalMeshAsset` (`self.SKM_ClothBottom`))
                (:`Is Not Valid`
                  (bind (_skeletalmesh_3 _masktexture_3) (`self.GetFashionDatas` "4"))
                  (`SkeletalMeshComponent.SetSkeletalMeshAsset` (`self.SKM_ClothBottom`) _skeletalmesh_3)
                  (`MaterialInstanceDynamic.SetTextureParameterValue` (`self.SkinMatRef`) "Mask Bottom" _masktexture_3))))))))))

(fn `Update Weapon Display`
  (params (HoldSocket :type Name))
  (locals (IsEquipBackpack :type Boolean))
  (bind _as_gi_battle_royale (`self.As GI Battle Royale`))
  (bind _as_gi_battle_royale_2 (`self.As GI Battle Royale`))
  (bind _weapon (`/Game/Blueprints/Gameplay/PS_BattleRoyale.GetWeapon1` (`self.As PS Battle Royale`)))
  (bind _weapon_2 (`/Game/Blueprints/Gameplay/PS_BattleRoyale.GetWeapon2` (`self.As PS Battle Royale`)))
  (bind _weapon_3 (`/Game/Blueprints/Gameplay/PS_BattleRoyale.GetHoldGun` (`self.As PS Battle Royale`)))
  (`|ExecutionSequence`
    (:`then_0`
      ;[0 1 0.9297] Update the handheld weapon display
      (if (!= (`local.HoldSocket`) "None")
        (`/Engine/EditorBlueprintResources/StandardMacros.IsValid` _weapon_3
          (:`Is Valid`
            (`self.Attach` _weapon_3 (`local.HoldSocket`))))))
    (:`then_1`
      ;[1 0.4688 0] Update back weapon display
      (`|ExecutionSequence`
        (:`then_0`
          (for _array_element (`/Game/Blueprints/Gameplay/PS_BattleRoyale.GetEquipments` (`self.As PS Battle Royale`))
            (if (`|EnumEquality` (`/Game/Blueprints/Items/ItemBase.ItemType` _array_element) "NewEnumerator7")
              (set `local.IsEquipBackpack` true))))
        (:`then_1`
          (`/Engine/EditorBlueprintResources/StandardMacros.IsValid` (`/Game/Blueprints/Gameplay/PS_BattleRoyale.GetWeapon1` (`self.As PS Battle Royale`))
            (:`Is Valid`
              (if (`local.IsEquipBackpack`)
                (`self.Attach` _weapon (`/Game/Blueprints/Gameplay/GI_BattleRoyale.BackLeftBName` _as_gi_battle_royale_2))
                (else
                  (`self.Attach` _weapon (`/Game/Blueprints/Gameplay/GI_BattleRoyale.BackLeftNName` _as_gi_battle_royale_2)))))))
        (:`then_2`
          (`/Engine/EditorBlueprintResources/StandardMacros.IsValid` (`/Game/Blueprints/Gameplay/PS_BattleRoyale.GetWeapon2` (`self.As PS Battle Royale`))
            (:`Is Valid`
              (if (`local.IsEquipBackpack`)
                (`self.Attach` _weapon_2 (`/Game/Blueprints/Gameplay/GI_BattleRoyale.BackRightBName` _as_gi_battle_royale))
                (else
                  (`self.Attach` _weapon_2 (`/Game/Blueprints/Gameplay/GI_BattleRoyale.BackRightNName` _as_gi_battle_royale)))))))))))

(fn `UpdateEquipmentDisplay`
  (locals (Item :type "/Game/Blueprints/Items/ItemBase Object Reference") (HasHelmet :type Boolean))
  (`|ExecutionSequence`
    (:`then_0`
      (for _array_element (`/Game/Blueprints/Gameplay/PS_BattleRoyale.GetEquipments` (`self.As PS Battle Royale`))
        (bind _output_get (set `local.Item` _array_element))
        (switch `/Game/Blueprints/Datas/Enum/E_ItemType` (`/Game/Blueprints/Items/ItemBase.ItemType` _output_get)
          (:`NewEnumerator5`
            (`self.Attach` (`local.Item`) (`/Game/Blueprints/Gameplay/GI_BattleRoyale.HelmetName` (`self.As GI Battle Royale`)))
            (set `local.HasHelmet` true))
          (:`NewEnumerator6`
            (`self.Attach` (`local.Item`) (`/Game/Blueprints/Gameplay/GI_BattleRoyale.VestName` (`self.As GI Battle Royale`))))
          (:`NewEnumerator7`
            (`self.Attach` (`local.Item`) (`/Game/Blueprints/Gameplay/GI_BattleRoyale.BackpackName` (`self.As GI Battle Royale`)))))))
    (:`then_1`
      (if (`local.HasHelmet`)
        (`SceneComponent.SetVisibility` (`self.SKM_Hair`) false false)
        (else
          (`SceneComponent.SetVisibility` (`self.SKM_Hair`) true false))))))

(fn `UpdateFashionDisplay`
  (`self.ClearFashion`)
  (for _array_element (`/Game/Blueprints/Gameplay/PS_BattleRoyale.GetFashions` (`self.As PS Battle Royale`))
    (bind _asitem_fashion (cast `/Game/Blueprints/Items/Equipment/ItemFashion` _array_element))
    (`self.ReplaceSkeletalMesh` (`/Game/Blueprints/Items/Equipment/ItemFashion.FashionType` _asitem_fashion) (`/Game/Blueprints/Items/ItemBase.ID` _asitem_fashion))))

(fn `UserConstructionScript`
  (`self.InitSkeletalMesh`))