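; Battle royale game mode that seeds world loot at BeginPlay and runs the shrinking safe zone, bombing and airdrops.
; GenerateItems fills data-table locations using percent-weighted random picks, adds matching ammo for weapons, and passes the pickups to player 0's controller.
; Safe zone stages come from DT_SafeZone, while GameInstance settings drive repeated bombing around player 0 and planes dropping random crates around the zone.
; Zone and bombing updates go to both HUD maps.
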(event `self.ReceiveBeginPlay`
  (set `self.As GI Battle Royale` (cast `/Game/Blueprints/Gameplay/GI_BattleRoyale` (`GameplayStatics.GetGameInstance`) :!pure true))
  (`|ExecutionSequence`
    (:`then_0`
      (bind _items (`self.GenerateItems`))
      (`/Game/Blueprints/Gameplay/PC_BattleRoyale.SetPickupItems` (cast `/Game/Blueprints/Gameplay/PC_BattleRoyale` (`GameplayStatics.GetPlayerController` 0) :!pure true) _items))
    (:`then_1`
      (`KismetSystemLibrary.Delay` 0.2)
      (`self.StartSafeZone`)
      (`self.StartBombing`))
    (:`then_2`
      (`self.StartAirdrop`))))

(event `StartSafeZone`
  ;[0.5234 1 0] The opening of the safe zone continues to shrink
  (bind _returnvalue (`|SpawnActorFromClass` "/Game/Blueprints/SafeZone/BP_SafeZone.BP_SafeZone_C" (`KismetMathLibrary.MakeTransform` (-66012.0 -160904.0 -6647.0)) "Undefined" "OverrideRootScale" null 500.0 null))
  (set `self.SafeZoneBP` _returnvalue)
  (`/Engine/EditorBlueprintResources/StandardMacros.IncrementInt` (`self.NumberOfTimes`) :!label _label
    (:`  `
      (bind (_isover_ _finalposition _finaldiameter _delaystartsec _duration _damage) (`self.RandomSafeZone`))
      (if (not _isover_)
        (set `self.SafeDamage` _damage)
        (`/Game/Blueprints/SafeZone/BP_SafeZone.StartToShrink` (`self.SafeZoneBP`) _finalposition _finaldiameter _delaystartsec _duration _damage)
        (`/Game/Blueprints/UI/Map/MapUI.UpdateSafeAreaState` (`/Game/Blueprints/UI/Map/BigMapArea.MapUI` (`/Game/Blueprints/Gameplay/HUD_BattleRoyale.BigMapUI` (cast `/Game/Blueprints/Gameplay/HUD_BattleRoyale` (`PlayerController.GetHUD` (`GameplayStatics.GetPlayerController` 0)) :!pure true))) _finaldiameter _finalposition)
        (`/Game/Blueprints/UI/Map/MapUI.UpdateSafeAreaState` (`/Game/Blueprints/UI/Map/SmallMapArea.MapUI` (`/Game/Blueprints/Gameplay/HUD_BattleRoyale.SmallMapUI` (cast `/Game/Blueprints/Gameplay/HUD_BattleRoyale` (`PlayerController.GetHUD` (`GameplayStatics.GetPlayerController` 0)) :!pure true))) _finaldiameter _finalposition)
        (`KismetSystemLibrary.Delay` (+ _delaystartsec _duration))
        (goto _label)))))

(event `StartAirdrop`
  ;[0 1 1] Turn on the airdrop
  (`KismetSystemLibrary.Delay` (`/Game/Blueprints/Gameplay/GI_BattleRoyale.AirdropIntervalTime` (`self.As GI Battle Royale`)) :!label _label_2)
  (bind _result (`/Engine/EditorBlueprintResources/StandardMacros.IncrementInt` (`self.Number`))
    (:`  `
      (if (<= _result (`/Game/Blueprints/Gameplay/GI_BattleRoyale.AirdropNumberOfTimes` (`self.As GI Battle Royale`)))
        (`|SpawnActorFromClass` "/Game/Blueprints/Airdrop/BP_AirdopPlane.BP_AirdopPlane_C" (`KismetMathLibrary.MakeTransform` (0.0 0.0 0.0)) "Undefined" "OverrideRootScale" null (`self.GetAirdropStart`) (`self.GetAirdropDrop`) (`self.GetAirdropItems`) null)
        (goto _label_2)))))

(event `StartBombing`
  (bind _as_gi_battle_royale (`self.As GI Battle Royale`))
  (`KismetArrayLibrary.Array_Clear` (`self.BombDatas`) :!label _label_3)
  (for _ (range 1 (+ (`/Game/Blueprints/Gameplay/GI_BattleRoyale.NumberOfBlasts` (`self.As GI Battle Royale`)) 1))
    (`KismetArrayLibrary.Array_Add` (`self.BombDatas`) (make `/Game/Blueprints/Datas/TableStructure/ST_BombZone` (+ (* (`KismetMathLibrary.MakeVector` (.x (`KismetMathLibrary.RandomUnitVectorInConeInDegrees` (0.0 0.0 1.0) 90.0)) (.y (`KismetMathLibrary.RandomUnitVectorInConeInDegrees` (0.0 0.0 1.0) 90.0))) (`/Game/Blueprints/Gameplay/GI_BattleRoyale.BombingRadius` (`self.As GI Battle Royale`))) (`self.K2_GetActorLocation` (`GameplayStatics.GetPlayerCharacter` 0))) (`KismetMathLibrary.RandomFloatInRange` 0.1 (`/Game/Blueprints/Gameplay/GI_BattleRoyale.DurationOfBlast` (`self.As GI Battle Royale`))))))
  (`|SpawnActorFromClass` "/Game/Blueprints/BombingArea/BombingArea.BombingArea_C" (`KismetMathLibrary.MakeTransform` (0.0 0.0 0.0)) "Undefined" "OverrideRootScale" null (`self.BombDatas`) (`/Game/Blueprints/Gameplay/GI_BattleRoyale.BombingInterval` (`self.As GI Battle Royale`)) null)
  (`/Game/Blueprints/UI/Map/MapUI.AddBombArea` (`/Game/Blueprints/UI/Map/BigMapArea.MapUI` (`/Game/Blueprints/Gameplay/HUD_BattleRoyale.BigMapUI` (cast `/Game/Blueprints/Gameplay/HUD_BattleRoyale` (`PlayerController.GetHUD` (`GameplayStatics.GetPlayerController` 0)) :!pure true))) (* (`/Game/Blueprints/Gameplay/GI_BattleRoyale.BombingRadius` (`self.As GI Battle Royale`)) 2.0) (`self.K2_GetActorLocation` (`GameplayStatics.GetPlayerCharacter` 0)))
  (`/Game/Blueprints/UI/Map/MapUI.AddBombArea` (`/Game/Blueprints/UI/Map/SmallMapArea.MapUI` (`/Game/Blueprints/Gameplay/HUD_BattleRoyale.SmallMapUI` (cast `/Game/Blueprints/Gameplay/HUD_BattleRoyale` (`PlayerController.GetHUD` (`GameplayStatics.GetPlayerController` 0)) :!pure true))) (* (`/Game/Blueprints/Gameplay/GI_BattleRoyale.BombingRadius` (`self.As GI Battle Royale`)) 2.0) (`self.K2_GetActorLocation` (`GameplayStatics.GetPlayerCharacter` 0)))
  (bind _result (`/Engine/EditorBlueprintResources/StandardMacros.IncrementInt` (`self.CurrentTime`))
    (:`  `
      (if (< _result (`/Game/Blueprints/Gameplay/GI_BattleRoyale.NumberOfBombing` (`self.As GI Battle Royale`)))
        (`KismetSystemLibrary.Delay` (+ (`/Game/Blueprints/Gameplay/GI_BattleRoyale.DurationOfBlast` _as_gi_battle_royale) (`/Game/Blueprints/Gameplay/GI_BattleRoyale.BombingInterval` _as_gi_battle_royale)))
        (goto _label_3)))))

(fn `GenerateItems`
  (returns (Items :type "Array of /Game/Blueprints/Items/Pickup/PickupBase Object Reference"))
  (locals (SpawnType :type "/Game/Blueprints/Datas/Enum/E_ItemType Enum") (SpawnID :type Name) (UsedLocation :type "Array of Transform Structure") (SpawnLocation :type "Transform Structure") (ItemsObject :type "Array of /Game/Blueprints/Items/Pickup/PickupBase Object Reference"))
  ;[1 0.7266 0] Get all itemgroup location
  (bind _outrownames (`DataTableFunctionLibrary.GetDataTableRowNames` "/Game/Blueprints/Datas/DataTable/Items/DT_ItemGroupLocation.DT_ItemGroupLocation"))
  (for _array_element _outrownames
    (bind _returnvalue (`|GetDataTableRow` "/Game/Blueprints/Datas/DataTable/Items/DT_ItemGroupLocation.DT_ItemGroupLocation" _array_element)
      (:`then`
        ;[1 0.5391 0] Spawn a Item Group Actor
        (bind _returnvalue_2 (`|SpawnActorFromClass` "/Game/Blueprints/Items/ItemGroup.ItemGroup_C" (`KismetMathLibrary.MakeTransform` (`.Location_2_7F58AD0D4A13D7AA524D838A1B8C8E39` (break `/Game/Blueprints/Datas/TableStructure/Items/ST_ItemGroupLocation` _returnvalue))) "Undefined" "OverrideRootScale" null null))
        (set `self.ItemGroupRef` _returnvalue_2)
        ;[0 1 0.1562] Number of random items
        (bind _number (`self.RandomItemNumber`))
        (for _ (range 1 (+ _number 1))
          ;[1 0 0.02387] Random Items Type
          (bind _itemtype (`self.RandomItemType` :!label _label))
          ;;[0.4062 1 0] Type cannot be  repeated
          (if (== (`KismetArrayLibrary.Array_Find` (`self.ItemsTypeArr`) _itemtype) -1)
            (`KismetArrayLibrary.Array_Add` (`self.ItemsTypeArr`) _itemtype)
            (else
              (goto _label))))
        ;[0.2656 0 1] Random items ID
        (for _array_element_2 (`self.ItemsTypeArr`)
          (bind _item (`self.RandomItemID` _array_element_2))
          (`KismetArrayLibrary.Array_Add` (`self.ItemsIDArr`) _item))
        ;[0.6406 0 1] If there are items of the weapon type, create a corresponding ammo item and remove the first item that is not a weapon
        (`KismetArrayLibrary.Array_Clear` (`self.ItemsTypeArr`))
        ;;[0.5039 1 0.3504] Find weapon item
        (for _array_element_3 (`self.ItemsIDArr`)
          (bind (_type _id) (break `/Game/Blueprints/Datas/TableStructure/ItemGeneration/ST_ItemTypeAndID` _array_element_3))
          (if (`|EnumEquality` _type "NewEnumerator0")
            ;;[0.2451 0.5043 1] Create a ammo
            (bind _returnvalue_3 (`|GetDataTableRow` "/Game/Blueprints/Datas/DataTable/Items/DT_Item_Weapon.DT_Item_Weapon" _id)
              (:`then`
                (`KismetArrayLibrary.Array_Add` (`self.ItemsIDArr`) (make `/Game/Blueprints/Datas/TableStructure/ItemGeneration/ST_ItemTypeAndID` "NewEnumerator2" (`.UseAmmoID_12_994AD0B848B6FCB8B28FDBB3B6E7A597` (break `/Game/Blueprints/Datas/TableStructure/Items/ST_Items_Weapon` _returnvalue_3))))
                ;;[0 0.8828 1] Remove a item
                (for (_array_element_4 _array_index) (`self.ItemsIDArr`)
                  (if (!= (`.Type_2_1B98F89E471442C3236B00876E203DE3` (break `/Game/Blueprints/Datas/TableStructure/ItemGeneration/ST_ItemTypeAndID` _array_element_4)) 0)
                    (`KismetArrayLibrary.Array_Remove` (`self.ItemsIDArr`) _array_index)
                    (break)))))))
        ;[1 0 0.07031] Loop all items ready to be generated
        (for _array_element_5 (`self.ItemsIDArr`)
          (bind (_type_2 _id_2) (break `/Game/Blueprints/Datas/TableStructure/ItemGeneration/ST_ItemTypeAndID` _array_element_5))
          (set `local.SpawnType` _type_2)
          (set `local.SpawnID` _id_2)
          (`|ExecutionSequence`
            (:`then_0`
              ;[1 0.375 0] Random Location
              (bind _location (`self.RandomLocation` (`/Game/Blueprints/Items/ItemGroup.GetAllTransform` (`self.ItemGroupRef`)) :!label _label_2))
              (if (== (`KismetArrayLibrary.Array_Find` (`local.UsedLocation`) _location) -1)
                (bind _output_get (set `local.SpawnLocation` _location))
                (`KismetArrayLibrary.Array_Add` (`local.UsedLocation`) _output_get)
                (else
                  (goto _label_2))))
            (:`then_1`
              ;[0 0.5312 1] Spawn Actor
              (switch `/Game/Blueprints/Datas/Enum/E_ItemType` (`local.SpawnType`)
                (:`NewEnumerator0`
                  ;;[0.6875 1 0] Spawn Weapon
                  (bind _returnvalue_4 (`|SpawnActorFromClass` "/Game/Blueprints/Items/Pickup/PickupWeapon.PickupWeapon_C" (`local.SpawnLocation`) "Undefined" "OverrideRootScale" null 0 (`local.SpawnID`) (`/Game/Blueprints/Gameplay/GI_BattleRoyale.GenerateSN` (`self.As GI Battle Royale`)) 1 null))
                  (`KismetArrayLibrary.Array_Add` (`local.ItemsObject`) _returnvalue_4))
                (:`NewEnumerator1`
                  ;;[0.7813 0 1] Spawn Accessories
                  (bind _returnvalue_5 (`|SpawnActorFromClass` "/Game/Blueprints/Items/Pickup/PickupWeaponAcc.PickupWeaponAcc_C" (`local.SpawnLocation`) "Undefined" "OverrideRootScale" null (`local.SpawnID`) (`/Game/Blueprints/Gameplay/GI_BattleRoyale.GenerateSN` (`self.As GI Battle Royale`)) 1 null))
                  (`KismetArrayLibrary.Array_Add` (`local.ItemsObject`) _returnvalue_5))
                (:`NewEnumerator2`
                  ;;[1 0.7266 0] Spawn Ammo
                  (bind _returnvalue_6 (`|SpawnActorFromClass` "/Game/Blueprints/Items/Pickup/PickupAmmo.PickupAmmo_C" (`local.SpawnLocation`) "Undefined" "OverrideRootScale" null (`local.SpawnID`) (`/Game/Blueprints/Gameplay/GI_BattleRoyale.GenerateSN` (`self.As GI Battle Royale`)) 0 null))
                  (`KismetArrayLibrary.Array_Add` (`local.ItemsObject`) _returnvalue_6))
                (:`NewEnumerator3`
                  ;;[1 0 0.375] Spawn Health
                  (bind _returnvalue_7 (`|SpawnActorFromClass` "/Game/Blueprints/Items/Pickup/PickupHealth.PickupHealth_C" (`local.SpawnLocation`) "Undefined" "OverrideRootScale" null (`local.SpawnID`) (`/Game/Blueprints/Gameplay/GI_BattleRoyale.GenerateSN` (`self.As GI Battle Royale`)) 1 null))
                  (`KismetArrayLibrary.Array_Add` (`local.ItemsObject`) _returnvalue_7))
                (:`NewEnumerator4`
                  ;;[0.1329 1 0] Spawn Boost
                  (bind _returnvalue_8 (`|SpawnActorFromClass` "/Game/Blueprints/Items/Pickup/PickupBoost.PickupBoost_C" (`local.SpawnLocation`) "Undefined" "OverrideRootScale" null (`local.SpawnID`) (`/Game/Blueprints/Gameplay/GI_BattleRoyale.GenerateSN` (`self.As GI Battle Royale`)) 1 null))
                  (`KismetArrayLibrary.Array_Add` (`local.ItemsObject`) _returnvalue_8))
                (:`NewEnumerator5`
                  ;;[1 0 0.09375] Spawn Equipment
                  (bind _returnvalue_9 (`|SpawnActorFromClass` "/Game/Blueprints/Items/Pickup/PickupEquipment.PickupEquipment_C" (`local.SpawnLocation`) "Undefined" "OverrideRootScale" null (`local.SpawnID`) (`/Game/Blueprints/Gameplay/GI_BattleRoyale.GenerateSN` (`self.As GI Battle Royale`)) 1 null :!label _label_3))
                  (`KismetArrayLibrary.Array_Add` (`local.ItemsObject`) _returnvalue_9))
                (:`NewEnumerator6`
                  (goto _label_3))
                (:`NewEnumerator7`
                  (goto _label_3))
                (:`NewEnumerator8`
                  ;;[1 0 0.375] Spawn Fashion
                  (bind _returnvalue_10 (`|SpawnActorFromClass` "/Game/Blueprints/Items/Pickup/PickupFashion.PickupFashion_C" (`local.SpawnLocation`) "Undefined" "OverrideRootScale" null (`local.SpawnID`) (`/Game/Blueprints/Gameplay/GI_BattleRoyale.GenerateSN` (`self.As GI Battle Royale`)) 1 null))
                  (`KismetArrayLibrary.Array_Add` (`local.ItemsObject`) _returnvalue_10))))))
        (`KismetArrayLibrary.Array_Clear` (`self.ItemsIDArr`)))))
  (return (`local.ItemsObject`)))

(fn `GetAirdropDrop`
  (returns (ReturnValue :type "Vector Structure"))
  (bind (_returnvalue_x _returnvalue_y) (`KismetMathLibrary.BreakVector` (`KismetMathLibrary.RandomUnitVectorInConeInDegrees` (0.0 0.0 1.0) 90.0)))
  (bind _finalscale_x (`KismetMathLibrary.BreakVector` (`/Game/Blueprints/SafeZone/BP_SafeZone.FinalScale` (`self.SafeZoneBP`))))
  (return (`KismetMathLibrary.MakeVector` (.x (+ (* (`KismetMathLibrary.MakeVector` _returnvalue_x _returnvalue_y) (* (/ _finalscale_x 2.0) 100.0)) (`/Game/Blueprints/SafeZone/BP_SafeZone.CurrentPosition` (`self.SafeZoneBP`)))) (.y (+ (* (`KismetMathLibrary.MakeVector` _returnvalue_x _returnvalue_y) (* (/ _finalscale_x 2.0) 100.0)) (`/Game/Blueprints/SafeZone/BP_SafeZone.CurrentPosition` (`self.SafeZoneBP`)))) 30000.0)))

(fn `GetAirdropItems`
  (returns (Items :type "Array of /Game/Blueprints/Datas/TableStructure/Airdrop/ST_AirdropBoxItem Structure"))
  (locals (AllItems :type "Array of /Game/Blueprints/Datas/TableStructure/Airdrop/ST_AirdropItems Structure") (ReturnItems :type "Array of /Game/Blueprints/Datas/TableStructure/Airdrop/ST_AirdropBoxItem Structure"))
  (bind (_itemtype _id _amount) (break `/Game/Blueprints/Datas/TableStructure/Airdrop/ST_AirdropItems` (`|GetArrayItem` (`local.AllItems`) (`KismetMathLibrary.RandomIntegerInRange` 0 99))))
  (bind _outrownames (`DataTableFunctionLibrary.GetDataTableRowNames` "/Game/Blueprints/Datas/DataTable/Airdrop/DT_AirdropItems.DT_AirdropItems"))
  (for _array_element _outrownames
    (bind _returnvalue (`|GetDataTableRow` "/Game/Blueprints/Datas/DataTable/Airdrop/DT_AirdropItems.DT_AirdropItems" _array_element)
      (:`then`
        (for _ (range 1 (+ (`.Percent_10_5A38D0C14FC18C1DB56DF2BC2BBD3198` (break `/Game/Blueprints/Datas/TableStructure/Airdrop/ST_AirdropItems` _returnvalue)) 1))
          (`KismetArrayLibrary.Array_Add` (`local.AllItems`) _returnvalue)))))
  (`KismetArrayLibrary.Array_Shuffle` (`local.AllItems`))
  (for _ (range 1 (+ (`/Game/Blueprints/Gameplay/GI_BattleRoyale.AirdropItemAmount` (`self.As GI Battle Royale`)) 1))
    (`KismetArrayLibrary.Array_Add` (`local.ReturnItems`) (make `/Game/Blueprints/Datas/TableStructure/Airdrop/ST_AirdropBoxItem` (`/Game/Blueprints/Gameplay/GI_BattleRoyale.GenerateSN` (`self.As GI Battle Royale`)) _itemtype _id _amount)))
  (return (`local.ReturnItems`)))

(fn `GetAirdropStart`
  (returns (ReturnValue :type "Vector Structure"))
  (bind _startingpoint (`self.RandomRoute`))
  (return (`KismetMathLibrary.MakeVector` (.x _startingpoint) (.y _startingpoint) 30000.0)))

(fn `RandomItemID`
  (params (ItemType :type "/Game/Blueprints/Datas/Enum/E_ItemType Enum" :default "NewEnumerator0"))
  (returns (Item :type "/Game/Blueprints/Datas/TableStructure/ItemGeneration/ST_ItemTypeAndID Structure"))
  (locals (Arr :type "Array of /Game/Blueprints/Datas/TableStructure/ItemGeneration/ST_ItemTypeAndID Structure"))
  (bind _arr (`local.Arr`))
  (`|ExecutionSequence`
    (:`then_0`
      (switch `/Game/Blueprints/Datas/Enum/E_ItemType` ItemType
        (:`NewEnumerator0`
          ;[0.7109 1 0] Weapons
          (bind _outrownames (`DataTableFunctionLibrary.GetDataTableRowNames` "/Game/Blueprints/Datas/DataTable/Items/DT_Item_Weapon.DT_Item_Weapon"))
          (for _array_element _outrownames
            (bind _returnvalue (`|GetDataTableRow` "/Game/Blueprints/Datas/DataTable/Items/DT_Item_Weapon.DT_Item_Weapon" _array_element)
              (:`then`
                (for _ (range 1 (+ (`.ProbabilityPercent_91_F0482D7F4A752BD06D69D5BCCE377529` (break `/Game/Blueprints/Datas/TableStructure/Items/ST_Items_Weapon` _returnvalue)) 1))
                  (`KismetArrayLibrary.Array_Add` (`local.Arr`) (make `/Game/Blueprints/Datas/TableStructure/ItemGeneration/ST_ItemTypeAndID` "NewEnumerator0" _array_element)))))))
        (:`NewEnumerator1`
          ;[1 0 0.3984] Accessories
          (bind _outrownames_2 (`DataTableFunctionLibrary.GetDataTableRowNames` "/Game/Blueprints/Datas/DataTable/Items/DT_Item_WeaponAcc.DT_Item_WeaponAcc"))
          (for _array_element_2 _outrownames_2
            (`KismetArrayLibrary.Array_Add` (`local.Arr`) (make `/Game/Blueprints/Datas/TableStructure/ItemGeneration/ST_ItemTypeAndID` "NewEnumerator1" _array_element_2))))
        (:`NewEnumerator2`
          ;[0.875 1 0] Ammo
          (bind _outrownames_3 (`DataTableFunctionLibrary.GetDataTableRowNames` "/Game/Blueprints/Datas/DataTable/Items/DT_Item_Ammo.DT_Item_Ammo"))
          (for _array_element_3 _outrownames_3
            (bind _returnvalue_2 (`|GetDataTableRow` "/Game/Blueprints/Datas/DataTable/Items/DT_Item_Ammo.DT_Item_Ammo" _array_element_3)
              (:`then`
                (for _ (range 1 (+ (`.ProbabilityPercent_17_8233BE66450A3F3BE0590694D8F2766D` (break `/Game/Blueprints/Datas/TableStructure/Items/ST_Item_Ammo` _returnvalue_2)) 1))
                  (`KismetArrayLibrary.Array_Add` (`local.Arr`) (make `/Game/Blueprints/Datas/TableStructure/ItemGeneration/ST_ItemTypeAndID` "NewEnumerator2" _array_element_3)))))))
        (:`NewEnumerator3`
          ;[0 1 0.0625] Health
          (bind _outrownames_4 (`DataTableFunctionLibrary.GetDataTableRowNames` "/Game/Blueprints/Datas/DataTable/Items/DT_Item_Health.DT_Item_Health"))
          (for _array_element_4 _outrownames_4
            (bind _returnvalue_3 (`|GetDataTableRow` "/Game/Blueprints/Datas/DataTable/Items/DT_Item_Health.DT_Item_Health" _array_element_4)
              (:`then`
                (for _ (range 1 (+ (`.ProbabilityPercent_21_8ADE87E447D2365F131BC1BCE6F0C92B` (break `/Game/Blueprints/Datas/TableStructure/Items/ST_Item_Health` _returnvalue_3)) 1))
                  (`KismetArrayLibrary.Array_Add` (`local.Arr`) (make `/Game/Blueprints/Datas/TableStructure/ItemGeneration/ST_ItemTypeAndID` "NewEnumerator3" _array_element_4)))))))
        (:`NewEnumerator4`
          ;[1 0.9375 0] Boost
          (bind _outrownames_5 (`DataTableFunctionLibrary.GetDataTableRowNames` "/Game/Blueprints/Datas/DataTable/Items/DT_Item_Boost.DT_Item_Boost"))
          (for _array_element_5 _outrownames_5
            (bind _returnvalue_4 (`|GetDataTableRow` "/Game/Blueprints/Datas/DataTable/Items/DT_Item_Boost.DT_Item_Boost" _array_element_5)
              (:`then`
                (for _ (range 1 (+ (`.ProbabilityPercent_19_0F2BD07C458E6C0F7D86AD80AE489328` (break `/Game/Blueprints/Datas/TableStructure/Items/ST_Item_Boost` _returnvalue_4)) 1))
                  (`KismetArrayLibrary.Array_Add` (`local.Arr`) (make `/Game/Blueprints/Datas/TableStructure/ItemGeneration/ST_ItemTypeAndID` "NewEnumerator4" _array_element_5)))))))
        (:`NewEnumerator5`
          ;[0 1 0.2266] Helmet
          (bind _outrownames_6 (`DataTableFunctionLibrary.GetDataTableRowNames` "/Game/Blueprints/Datas/DataTable/Items/DT_Item_Equipment.DT_Item_Equipment"))
          (for _array_element_6 _outrownames_6
            (bind _returnvalue_5 (`|GetDataTableRow` "/Game/Blueprints/Datas/DataTable/Items/DT_Item_Equipment.DT_Item_Equipment" _array_element_6)
              (:`then`
                (bind ((`Type_5_DC24227D41F076E3293BD5B6B6CD5E1C` _type) (`ProbabilityPercent_19_7C23C8F94531A466940C45927D8E83C3` _probabilitypercent)) (break `/Game/Blueprints/Datas/TableStructure/Items/ST_Item_Equipment` _returnvalue_5))
                (if (`|EnumEquality` _type "NewEnumerator5")
                  (for _ (range 1 (+ _probabilitypercent 1))
                    (`KismetArrayLibrary.Array_Add` (`local.Arr`) (make `/Game/Blueprints/Datas/TableStructure/ItemGeneration/ST_ItemTypeAndID` "NewEnumerator5" _array_element_6))))))))
        (:`NewEnumerator6`
          ;[0.5 0 1] Vest
          (bind _outrownames_7 (`DataTableFunctionLibrary.GetDataTableRowNames` "/Game/Blueprints/Datas/DataTable/Items/DT_Item_Equipment.DT_Item_Equipment"))
          (for _array_element_7 _outrownames_7
            (bind _returnvalue_6 (`|GetDataTableRow` "/Game/Blueprints/Datas/DataTable/Items/DT_Item_Equipment.DT_Item_Equipment" _array_element_7)
              (:`then`
                (bind ((`Type_5_DC24227D41F076E3293BD5B6B6CD5E1C` _type_2) (`ProbabilityPercent_19_7C23C8F94531A466940C45927D8E83C3` _probabilitypercent_2)) (break `/Game/Blueprints/Datas/TableStructure/Items/ST_Item_Equipment` _returnvalue_6))
                (if (`|EnumEquality` _type_2 "NewEnumerator6")
                  (for _ (range 1 (+ _probabilitypercent_2 1))
                    (`KismetArrayLibrary.Array_Add` (`local.Arr`) (make `/Game/Blueprints/Datas/TableStructure/ItemGeneration/ST_ItemTypeAndID` "NewEnumerator6" _array_element_7))))))))
        (:`NewEnumerator7`
          ;[1 0.6563 0] Backpack
          (bind _outrownames_8 (`DataTableFunctionLibrary.GetDataTableRowNames` "/Game/Blueprints/Datas/DataTable/Items/DT_Item_Equipment.DT_Item_Equipment"))
          (for _array_element_8 _outrownames_8
            (bind _returnvalue_7 (`|GetDataTableRow` "/Game/Blueprints/Datas/DataTable/Items/DT_Item_Equipment.DT_Item_Equipment" _array_element_8)
              (:`then`
                (bind ((`Type_5_DC24227D41F076E3293BD5B6B6CD5E1C` _type_3) (`ProbabilityPercent_19_7C23C8F94531A466940C45927D8E83C3` _probabilitypercent_3)) (break `/Game/Blueprints/Datas/TableStructure/Items/ST_Item_Equipment` _returnvalue_7))
                (if (`|EnumEquality` _type_3 "NewEnumerator7")
                  (for _ (range 1 (+ _probabilitypercent_3 1))
                    (`KismetArrayLibrary.Array_Add` (`local.Arr`) (make `/Game/Blueprints/Datas/TableStructure/ItemGeneration/ST_ItemTypeAndID` "NewEnumerator7" _array_element_8))))))))
        (:`NewEnumerator8`
          ;[0.007812 1 0] Fashion
          (bind _outrownames_9 (`DataTableFunctionLibrary.GetDataTableRowNames` "/Game/Blueprints/Datas/DataTable/Items/DT_Item_Fashion.DT_Item_Fashion"))
          (for _array_element_9 _outrownames_9
            (if (and (!= _array_element_9 "1") (!= _array_element_9 "4"))
              (`KismetArrayLibrary.Array_Add` (`local.Arr`) (make `/Game/Blueprints/Datas/TableStructure/ItemGeneration/ST_ItemTypeAndID` "NewEnumerator8" _array_element_9)))))))
    (:`then_1`
      ;[1 0 0.7969] Random and Shuffle Number
      (`KismetArrayLibrary.Array_Shuffle` _arr)
      (return (`|GetArrayItem` _arr (`KismetMathLibrary.RandomIntegerInRange` 0 (- (`KismetArrayLibrary.Array_Length` (`local.Arr`)) 1)))))))

(fn `RandomItemNumber`
  (returns (Number :type Integer))
  (locals (Arr :type "Array of Integer"))
  (bind _arr (`local.Arr`))
  (bind _outrownames (`DataTableFunctionLibrary.GetDataTableRowNames` "/Game/Blueprints/Datas/DataTable/ItemGeneration/DT_NumberProbability.DT_NumberProbability"))
  (for _array_element _outrownames
    (bind _returnvalue (`|GetDataTableRow` "/Game/Blueprints/Datas/DataTable/ItemGeneration/DT_NumberProbability.DT_NumberProbability" _array_element)
      (:`then`
        (bind (_percent _number) (break `/Game/Blueprints/Datas/TableStructure/ItemGeneration/ST_NumberProbability` _returnvalue))
        (for _ (range (+ _percent 1))
          (`KismetArrayLibrary.Array_Add` (`local.Arr`) _number)))))
  (`KismetArrayLibrary.Array_Shuffle` _arr)
  (return (`|GetArrayItem` _arr (`KismetMathLibrary.RandomIntegerInRange` 0 99))))

(fn `RandomItemType`
  (returns (ItemType :type "/Game/Blueprints/Datas/Enum/E_ItemType Enum"))
  (locals (Arr :type "Array of /Game/Blueprints/Datas/Enum/E_ItemType Enum"))
  (bind _arr (`local.Arr`))
  (bind _outrownames (`DataTableFunctionLibrary.GetDataTableRowNames` "/Game/Blueprints/Datas/DataTable/ItemGeneration/DT_ItemTypeProbability.DT_ItemTypeProbability"))
  (for _array_element _outrownames
    (bind _returnvalue (`|GetDataTableRow` "/Game/Blueprints/Datas/DataTable/ItemGeneration/DT_ItemTypeProbability.DT_ItemTypeProbability" _array_element)
      (:`then`
        (bind (_percent _type) (break `/Game/Blueprints/Datas/TableStructure/ItemGeneration/ST_ItemTypeProbability` _returnvalue))
        (for _ (range (+ _percent 1))
          (`KismetArrayLibrary.Array_Add` (`local.Arr`) _type)))))
  (`KismetArrayLibrary.Array_Shuffle` _arr)
  (return (`|GetArrayItem` _arr (`KismetMathLibrary.RandomIntegerInRange` 0 99))))

(fn `RandomLocation`
  (params (Available :type "Array of Transform Structure"))
  (returns (Location :type "Transform Structure"))
  (return (`|GetArrayItem` Available (`KismetMathLibrary.RandomIntegerInRange` 0 (- (`KismetArrayLibrary.Array_Length` Available) 1)))))

(fn `RandomRoute`
  (returns (StartingPoint :type "Vector Structure") (EndPoint :type "Vector Structure"))
  (locals (StartIndex :type Integer :default 0) (LineMin :type "Vector2D Structure") (LineMax :type "Vector2D Structure") (StartVector :type "Vector Structure") (EndIndex :type Integer) (EndVector :type "Vector Structure"))
  (bind _startindex (`local.StartIndex`))
  (bind _as_gi_battle_royale (`self.As GI Battle Royale`))
  (bind _as_gi_battle_royale_2 (`self.As GI Battle Royale`))
  (bind _endindex (`local.EndIndex`))
  (bind _as_gi_battle_royale_3 (`self.As GI Battle Royale`))
  (bind _as_gi_battle_royale_4 (`self.As GI Battle Royale`))
  (bind _as_gi_battle_royale_5 (`self.As GI Battle Royale`))
  (bind _as_gi_battle_royale_6 (`self.As GI Battle Royale`))
  (bind _as_gi_battle_royale_7 (`self.As GI Battle Royale`))
  (bind _as_gi_battle_royale_8 (`self.As GI Battle Royale`))
  (bind (_x _y) (`KismetMathLibrary.BreakVector2D` (`local.LineMax`)))
  (bind (_x_2 _y_2) (`KismetMathLibrary.BreakVector2D` (`local.LineMax`)))
  (bind (_x_3 _y_3) (`KismetMathLibrary.BreakVector2D` (`local.LineMin`)))
  (bind (_x_4 _y_4) (`KismetMathLibrary.BreakVector2D` (`local.LineMin`)))
  (`|ExecutionSequence`
    (:`then_0`
      ;[0.5234 0 1] Random Start
      (`|ExecutionSequence`
        (:`then_0`
          (set `local.StartIndex` (`KismetMathLibrary.RandomIntegerInRange` 1 4))
          (if (== _startindex 1)
            (set `local.LineMin` (`/Game/Blueprints/Gameplay/GI_BattleRoyale.Line1Min` _as_gi_battle_royale_3))
            (set `local.LineMax` (`/Game/Blueprints/Gameplay/GI_BattleRoyale.Line1Max` _as_gi_battle_royale_3))
            (elif (== _startindex 2)
              (set `local.LineMin` (`/Game/Blueprints/Gameplay/GI_BattleRoyale.Line2Min` _as_gi_battle_royale_4))
              (set `local.LineMax` (`/Game/Blueprints/Gameplay/GI_BattleRoyale.Line2Max` _as_gi_battle_royale_4))
              (elif (== _startindex 3)
                (set `local.LineMin` (`/Game/Blueprints/Gameplay/GI_BattleRoyale.Line3Min` _as_gi_battle_royale_5))
                (set `local.LineMax` (`/Game/Blueprints/Gameplay/GI_BattleRoyale.Line3Max` _as_gi_battle_royale_5))
                (else
                  (set `local.LineMin` (`/Game/Blueprints/Gameplay/GI_BattleRoyale.Line4Min` _as_gi_battle_royale_6))
                  (set `local.LineMax` (`/Game/Blueprints/Gameplay/GI_BattleRoyale.Line4Max` _as_gi_battle_royale_6)))))))
        (:`then_1`
          (set `local.StartVector` (`KismetMathLibrary.MakeVector` (`KismetMathLibrary.RandomFloatInRange` _x_4 _x) (`KismetMathLibrary.RandomFloatInRange` _y_4 _y) 150000.0)))))
    (:`then_1`
      ;[1 0.8672 0] Random End
      (`|ExecutionSequence`
        (:`then_0`
          ;;[0 0.25 1] Cannot be the same side as the starting point
          (bind _output_get (set `local.EndIndex` (`KismetMathLibrary.RandomIntegerInRange` 0) :!label _label))
          (if (== _output_get (`local.StartIndex`))
            (goto _label)
            (elif (== _endindex 1)
              (set `local.LineMin` (`/Game/Blueprints/Gameplay/GI_BattleRoyale.Line1Min` _as_gi_battle_royale_7))
              (set `local.LineMax` (`/Game/Blueprints/Gameplay/GI_BattleRoyale.Line1Max` _as_gi_battle_royale_7))
              (elif (== _endindex 2)
                (set `local.LineMin` (`/Game/Blueprints/Gameplay/GI_BattleRoyale.Line2Min` _as_gi_battle_royale_8))
                (set `local.LineMax` (`/Game/Blueprints/Gameplay/GI_BattleRoyale.Line2Max` _as_gi_battle_royale_8))
                (elif (== _endindex 3)
                  (set `local.LineMin` (`/Game/Blueprints/Gameplay/GI_BattleRoyale.Line3Min` _as_gi_battle_royale_2))
                  (set `local.LineMax` (`/Game/Blueprints/Gameplay/GI_BattleRoyale.Line3Max` _as_gi_battle_royale_2))
                  (else
                    (set `local.LineMin` (`/Game/Blueprints/Gameplay/GI_BattleRoyale.Line4Min` _as_gi_battle_royale))
                    (set `local.LineMax` (`/Game/Blueprints/Gameplay/GI_BattleRoyale.Line4Max` _as_gi_battle_royale))))))))
        (:`then_1`
          (set `local.EndVector` (`KismetMathLibrary.MakeVector` (`KismetMathLibrary.RandomFloatInRange` _x_3 _x_2) (`KismetMathLibrary.RandomFloatInRange` _y_3 _y_2) 150000.0)))))
    (:`then_2`
      (return (`local.StartVector`) (`local.EndVector`)))))

(fn `RandomSafeZone`
  (returns (`IsOver?` :type Boolean) (FinalPosition :type "Vector Structure") (FinalDiameter :type "Float (double-precision)") (DelayStartSec :type "Float (double-precision)") (Duration :type "Float (double-precision)") (Damage :type "Float (double-precision)"))
  (locals (Diameter :type "Float (double-precision)"))
  (bind (_returnvalue_x _returnvalue_y) (`KismetMathLibrary.BreakVector` (`KismetMathLibrary.RandomUnitVectorInConeInDegrees` (0.0 0.0 1.0) 90.0)))
  (bind _position (`/Game/Blueprints/SafeZone/BP_SafeZone.CurrentPosition` (`self.SafeZoneBP`)))
  (bind _finalscale_x (`KismetMathLibrary.BreakVector` (`/Game/Blueprints/SafeZone/BP_SafeZone.FinalScale` (`self.SafeZoneBP`))))
  ;[1 0.2344 0] The final diameter after reduction
  (bind _returnvalue (`|GetDataTableRow` "/Game/Blueprints/Datas/DataTable/DT_SafeZone.DT_SafeZone" (`KismetStringLibrary.Conv_StringToName` (`KismetStringLibrary.Conv_IntToString` (`self.NumberOfTimes`))))
    (:`then`
      (bind (_delayedstartsec _duration _scaling _damage) (break `/Game/Blueprints/Datas/TableStructure/ST_SafeZone` _returnvalue))
      (set `local.Diameter` (* _finalscale_x _scaling))
      (return false (`KismetMathLibrary.MakeVector` (.x (+ (* (`KismetMathLibrary.MakeVector` _returnvalue_x _returnvalue_y) (* (/ (`local.Diameter`) 2.0) 100.0)) _position)) (.y (+ (* (`KismetMathLibrary.MakeVector` _returnvalue_x _returnvalue_y) (* (/ (`local.Diameter`) 2.0) 100.0)) _position)) (.z _position)) (`local.Diameter`) _delayedstartsec _duration _damage))
    (:`RowNotFound`
      (return true (0.0 0.0 0.0) 0.0 0.0 0.0 0.0))))

(fn `UserConstructionScript`)