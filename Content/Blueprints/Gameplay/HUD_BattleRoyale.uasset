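; Battle royale HUD that creates the in-game widgets on BeginPlay and adds them to the viewport.
; Crosshairs, user info, countdown, direction and small map start on screen, while action tips, message tips, item use, parachute and big map start hidden.
; Stored widget references back Show/Hide functions for action tips, item use and parachute, passing in text or a timer.
; Message tips only has a Show function.
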(event `self.ReceiveBeginPlay`
  (`|ExecutionSequence`
    (:`then_0`
      (bind _returnvalue (`|CreateWidget` "/Game/Blueprints/UI/MainUI/CrosshairsUI.CrosshairsUI_C"))
      (`UserWidget.AddToViewport` _returnvalue 0))
    (:`then_1`
      (bind _returnvalue_2 (`|CreateWidget` "/Game/Blueprints/UI/MainUI/ActiontTipsUI.ActiontTipsUI_C"))
      (bind _output_get (set `self.ActionTipsUI` _returnvalue_2))
      (`Widget.SetVisibility` _output_get "Hidden")
      (`UserWidget.AddToViewport` _output_get 0))
    (:`then_2`
      (bind _returnvalue_3 (`|CreateWidget` "/Game/Blueprints/UI/MainUI/MessageTipsUI.MessageTipsUI_C"))
      (bind _output_get_2 (set `self.MessageTipsUI` _returnvalue_3))
      (`Widget.SetVisibility` _output_get_2 "Hidden")
      (`UserWidget.AddToViewport` _output_get_2 1))
    (:`then_3`
      (bind _returnvalue_4 (`|CreateWidget` "/Game/Blueprints/UI/MainUI/UserInfoUI.UserInfoUI_C"))
      (bind _output_get_3 (set `self.UserInfoUI` _returnvalue_4))
      (`UserWidget.AddToViewport` _output_get_3 0))
    (:`then_4`
      (bind _returnvalue_5 (`|CreateWidget` "/Game/Blueprints/UI/MainUI/CountdownUI.CountdownUI_C"))
      (`UserWidget.AddToViewport` _returnvalue_5 0))
    (:`then_5`
      (bind _returnvalue_6 (`|CreateWidget` "/Game/Blueprints/UI/MainUI/DirectionUI.DirectionUI_C"))
      (`UserWidget.AddToViewport` _returnvalue_6 0))
    (:`then_6`
      (bind _returnvalue_7 (`|CreateWidget` "/Game/Blueprints/UI/MainUI/UseItemUI.UseItemUI_C"))
      (bind _output_get_4 (set `self.UseItemUI` _returnvalue_7))
      (`Widget.SetVisibility` _output_get_4 "Hidden")
      (`UserWidget.AddToViewport` _output_get_4 1))
    (:`then_7`
      (bind _returnvalue_8 (`|CreateWidget` "/Game/Blueprints/UI/Parachute/ParachuteUI.ParachuteUI_C"))
      (bind _output_get_5 (set `self.ParachuteUI` _returnvalue_8))
      (`Widget.SetVisibility` _output_get_5 "Hidden")
      (`UserWidget.AddToViewport` _output_get_5 0))
    (:`then_8`
      (bind _returnvalue_9 (`|CreateWidget` "/Game/Blueprints/UI/Map/BigMapArea.BigMapArea_C"))
      (bind _output_get_6 (set `self.BigMapUI` _returnvalue_9))
      (`Widget.SetVisibility` _output_get_6 "Hidden")
      (`UserWidget.AddToViewport` _output_get_6 0)
      (bind _returnvalue_10 (`|CreateWidget` "/Game/Blueprints/UI/Map/SmallMapArea.SmallMapArea_C"))
      (bind _output_get_7 (set `self.SmallMapUI` _returnvalue_10))
      (`Widget.SetVisibility` _output_get_7 "Visible")
      (`UserWidget.AddToViewport` _output_get_7 0))))

(fn `HideActionTipsUI`
  (`Widget.SetVisibility` (`self.ActionTipsUI`) "Hidden"))

(fn `HideParachuteUI`
  (`Widget.SetVisibility` (`self.ParachuteUI`) "Hidden"))

(fn `HideUseItemUI`
  (`Widget.SetVisibility` (`self.UseItemUI`) "Hidden"))

(fn `ShowActionTipsUI`
  (params (Info :type Text))
  (`/Game/Blueprints/UI/MainUI/ActiontTipsUI.SetInfo` (`self.ActionTipsUI`) Info)
  (`Widget.SetVisibility` (`self.ActionTipsUI`) "Visible"))

(fn `ShowMessageTipsUI`
  (params (Info :type Text))
  (`/Game/Blueprints/UI/MainUI/MessageTipsUI.SetInfo` (`self.MessageTipsUI`) Info)
  (`Widget.SetVisibility` (`self.MessageTipsUI`) "Visible"))

(fn `ShowParachuteUI`
  (`Widget.SetVisibility` (`self.ParachuteUI`) "Visible"))

(fn `ShowUseItemUI`
  (params (Time :type "Float (double-precision)"))
  (`/Game/Blueprints/UI/MainUI/UseItemUI.Start` (`self.UseItemUI`) Time)
  (`Widget.SetVisibility` (`self.UseItemUI`) "Visible"))

(fn `UserConstructionScript`)