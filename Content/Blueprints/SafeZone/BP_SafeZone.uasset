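; BP_SafeZone is a safe zone actor whose tall static mesh moves and narrows to a given position and diameter.
; The construction script sizes it from InitDiameter.
; StartToShrink caches start and target transforms, waits a delay, then lerps location and XY scale on a timeline stretched to the requested duration, destroying the actor when the final diameter is zero.
; Despite its name, CurrentPosition returns the target diameter.
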(event `StartToShrink`
  (params (FinalPosition :type "Vector Structure") (FinalDiameter :type "Float (double-precision)") (DelayedStartSec :type "Float (double-precision)") (Duration :type "Float (double-precision)"))
  (bind _finalscale_x (`KismetMathLibrary.BreakVector` (`self.FinalScale`)))
  (bind _returnvalue (`SceneComponent.K2_GetComponentScale` (`self.StaticMesh`)))
  ;[0 1 1] Start narrowing the safety zone
  (`|ExecutionSequence`
    (:`then_0`
      ;;[0.7344 1 0] Save the datas
      (set `self.StartPostion` (`self.K2_GetActorLocation`))
      (set `self.FinalPosition` FinalPosition)
      (set `self.StartScale` _returnvalue)
      (set `self.FinalScale` (`KismetMathLibrary.MakeVector` FinalDiameter FinalDiameter (`.Z` (`KismetMathLibrary.BreakVector3f` _returnvalue)))))
    (:`then_1`
      ;;[0.1016 0 1] Narrow the safety zone
      (`KismetSystemLibrary.Delay` DelayedStartSec)
      (`TimelineComponent.SetTimelineLength` (`self.Timeline_Shrink`) Duration)
      (bind (_direction _time) (`Timeline|Timeline_Shrink` :!via `PlayFromStart`)
        (:`Update`
          (bind _returnvalue_2 (/ _time Duration))
          (`self.K2_SetActorLocation` (`KismetMathLibrary.VLerp` (`self.StartPostion`) (`self.FinalPosition`) _returnvalue_2))
          (`SceneComponent.SetWorldScale3D` (`self.StaticMesh`) (`KismetMathLibrary.VLerp` (`self.StartScale`) (`self.FinalScale`) _returnvalue_2)))
        (:`Finished`
          (if (== _finalscale_x 0.0)
            (`self.K2_DestroyActor`)))))))

(fn `CurrentPosition`
  (returns (Diameter :type "Float (double-precision)"))
  (bind _finalscale_x (`KismetMathLibrary.BreakVector` (`self.FinalScale`)))
  (return _finalscale_x))

(fn `UserConstructionScript`
  (bind _initdiameter (`self.InitDiameter`))
  (`SceneComponent.SetWorldScale3D` (`self.StaticMesh`) (`KismetMathLibrary.MakeVector` _initdiameter _initdiameter 10000.0))
  (set `self.FinalScale` (`KismetMathLibrary.MakeVector` _initdiameter _initdiameter))
  (set `self.FinalPosition` (`self.K2_GetActorLocation`)))